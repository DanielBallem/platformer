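; BouncePad is an actor that launches any Character that hits it along the direction of its arrow component.
; On BeginPlay it looks up its pad type's row in a data table to set launch power and sphere material, falling back to a debug material if no row matches.
; On hit, the launch overrides the character's vertical velocity and adds to its horizontal velocity.
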(event Collision|EventHit
  (params (MyComp :type Primitive%20Component%20Object%20Reference) (Other :type Actor%20Object%20Reference) (OtherComp :type Primitive%20Component%20Object%20Reference) (bSelfMoved :type Boolean) (HitLocation :type Vector :default "0, 0, 0") (HitNormal :type Vector :default "0, 0, 0") (NormalImpulse :type Vector :default "0, 0, 0") (Hit :type Hit%20Result%20Structure%20%28by%20ref%29))
  (bind _ascharacter (Utilities|Casting|CastToCharacter Other))
  (Character|LaunchCharacter _ascharacter (* (Math|Vector|GetForwardVector (Variables|Default|GetArrow)) (Variables|Default|GetLaunchPowerMultiplyer)) false true))

(event EventBeginPlay
  (bind _sphere (Variables|Default|GetSphere))
  (bind _returnvalue (Utilities|GetDataTableRow "/Game/Data/BouncePadDataTable.BouncePadDataTable" (Utilities|String|StringToName (Utilities|String|EnumtoString (Variables|Default|GetBouncePadType))))
    (:then
      (Variables|Default|SetLaunchPowerMultiplyer (.powermultiplyer _returnvalue))
      (Rendering|Material|SetMaterial _sphere 0 (.material _returnvalue)))
    (:RowNotFound
      (Rendering|Material|SetMaterial _sphere 0 "/Game/Materials/DebugMat.DebugMat"))))

(fn ConstructionScript)