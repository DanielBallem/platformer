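; A collectable pickup actor that destroys itself when the third-person character or an Enemy overlaps it.
; Its mesh comes from a configurable reference, applied in the construction script and again at BeginPlay.
; SnapFromFloor traces down on the Visibility channel and places the root at a set height above the hit, in both passes.
; BeginPlay then switches bounding box physics simulation according to the GravityEnabled flag.
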(event EventBeginPlay
  (Components|StaticMesh|SetStaticMesh (Variables|Default|GetCollectableMesh) (Variables|Default|GetcollectableMeshReference))
  (CallFunction|SnapfromFloor)
  (Physics|SetSimulatePhysics (Variables|Default|GetboundingBox) (Variables|Default|GetgravityEnabled)))

(event Collision|EventActorBeginOverlap
  (params (OtherActor :type Actor%20Object%20Reference))
  (Utilities|Casting|CastToBP_ThirdPersonCharacter OtherActor
    (:then
      _)
    (:CastFailed
      (Utilities|Casting|CastToEnemy OtherActor)))
  (Actor|DestroyActor))

(event EventTick
  (params (DeltaSeconds :type Float%20%28single-precision%29)))

(fn ConstructionScript
  (Components|StaticMesh|SetStaticMesh (Variables|Default|GetCollectableMesh) (Variables|Default|GetcollectableMeshReference))
  (CallFunction|SnapfromFloor))

(fn SnapfromFloor
  (bind _collectablemesh (Variables|Default|GetCollectableMesh))
  (bind _returnvalue (Transformation|GetWorldLocation _collectablemesh))
  (bind (_outhit _returnvalue_2) (Collision|LineTraceByChannel _returnvalue (+ _returnvalue (* (Math|Vector|VectorDown) (Variables|Default|GetsnapDistance))) "TraceTypeQuery1" false 0 "None"))
  (if _returnvalue_2
    (Transformation|SetWorldLocation (Variables|Default|GetDefaultSceneRoot) (+ (.location _outhit) (* (Math|Vector|VectorUp) (Variables|Default|GetsnapToDistance))) false true)))