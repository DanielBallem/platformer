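; CommonCollectableBP is a collectable actor that animates its mesh with a hovering and spinning motion.
; On BeginPlay it starts a timeline at HoverOffset, so the animation phase can be shifted.
; Each update adds the hover track, scaled by HoverMultiplier, to the mesh's current height and sets world yaw from the rotation track.
; It contains no pickup logic, as overlap and tick events are disabled.
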(event EventBeginPlay
  (bind _collectablemesh (Variables|Default|GetCollectableMesh))
  (|CallParentFunction)
  (Components|Timeline|SetNewTime (Variables|Default|GetCommon%20Collectable%20T) (Variables|Default|GethoverOffset))
  (bind (_direction _hovertrack _rotationtrack) (Timeline|Common%20Collectable%20T Play)
    (:Update
      (Transformation|SetWorldLocation _collectablemesh (+ (Transformation|GetWorldLocation (Variables|Default|GetCollectableMesh)) (* (Math|Vector|VectorUp) (* _hovertrack (Variables|Default|GethoverMultiplier)))) false false)
      (Transformation|SetWorldRotation _collectablemesh (Math|Rotator|MakeRotator 0.0 0.0 (* _rotationtrack 3.6e+02)) false false))))

(event Collision|EventActorBeginOverlap
  (params (OtherActor :type Actor%20Object%20Reference))
  (|CallParentFunction OtherActor) ; This node is disabled and will not be called.\nDrag off pins to build functionality.
)

(event EventTick
  (params (DeltaSeconds :type Float%20%28single-precision%29))
  (|CallParentFunction DeltaSeconds) ; This node is disabled and will not be called.\nDrag off pins to build functionality.
)

(fn ConstructionScript
  (|CallParentFunction))