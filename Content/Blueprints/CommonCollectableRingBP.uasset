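; Blueprint actor that spawns a ring of collectables around itself on BeginPlay.
; SpawnCollectables rotates the root's forward vector around its up vector in equal angular steps, scales it by the radius and spawns the configured class there.
; TotalDegrees sets the arc, and CollectablesMinus trims the loop's last index.
; The construction script sizes an arrow component to the circle radius.
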(event EventBeginPlay
  (CallFunction|SpawnCollectables))

(event Collision|EventActorBeginOverlap
  (params (OtherActor :type Actor%20Object%20Reference)))

(event EventTick
  (params (DeltaSeconds :type Float%20%28single-precision%29)))

(fn ConstructionScript
  (Variables|/Script/Engine.ArrowComponent|SetArrowLength (Variables|Default|GetArrow) (Variables|Default|GetCircleRadius)))

(fn SpawnCollectables
  (bind _numberofcollectables (Variables|Default|GetNumberOfCollectables))
  (bind _defaultsceneroot (Variables|Default|GetDefaultSceneRoot))
  (for _index (range 0 (- _numberofcollectables (Variables|Default|GetcollectablesMinus)))
    (Game|SpawnActorfromClass (Variables|Default|GetCollectableToSpawn) (Math|Conversions|ToTransform(Vector) (+ (* (Math|Vector|RotateVectorAroundAxis (Math|Vector|GetForwardVector _defaultsceneroot) (* (/ (Variables|Default|GetTotalDegrees) _numberofcollectables) _index) (Math|Vector|GetUpVector _defaultsceneroot)) (Variables|Default|GetCircleRadius)) (Transformation|GetWorldLocation (Variables|Default|GetDefaultSceneRoot)))) "Undefined" "MultiplyWithRoot" 0 0.0 0)))