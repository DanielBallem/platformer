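; CommonCollectableSet is an actor that lays out a row of CommonCollectableBP pickups along its spline when play begins.
; SpawnCollectables spaces them evenly by dividing spline length by NumberOfCollectables, with CollectablesMinus reducing the loop's last index.
; Each pickup receives a HoverOffset proportional to its index, staggering that value along the set.
; Each iteration also adds a child actor component after spawning.
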(event EventBeginPlay
  (CallFunction|SpawnCollectables))

(event Collision|EventActorBeginOverlap
  (params (OtherActor :type Actor%20Object%20Reference)))

(event EventTick
  (params (DeltaSeconds :type Float%20%28single-precision%29)))

(fn ConstructionScript)

(fn SpawnCollectables
  (bind _spline (Variables|Default|GetSpline))
  (bind _numberofcollectables (Variables|Default|GetNumberOfCollectables))
  (bind _collectablesminus (Variables|Default|GetcollectablesMinus))
  (bind _returnvalue (- _numberofcollectables _collectablesminus))
  (for _index (range 0 _returnvalue)
    (Game|SpawnActorfromClass "/Game/Blueprints/CommonCollectableBP.CommonCollectableBP_C" (Math|Conversions|ToTransform(Vector) (Spline|GetLocationatDistanceAlongSpline _spline (* (/ (Spline|GetSplineLength _spline) _numberofcollectables) _index) "World")) "Undefined" "MultiplyWithRoot" 0 (/ (Math|Conversions|ToFloat(Integer) _index) (Math|Conversions|ToFloat(Integer) _returnvalue)) 0)
    (AddComponent|AddChildActorComponent false)))