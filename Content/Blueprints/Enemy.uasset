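; Enemy character that turns into a bouncing projectile when it registers a hit while its character movement is active.
; Character and projectile movement are mutually exclusive, with projectile movement switched off at BeginPlay.
; The hit swaps the active component and launches the enemy horizontally away from the other component at a fixed speed scale.
; Each bounce increments a counter until the bounce limit is reached, then the next bounce destroys the actor.
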(event OnProjectileBounce(ProjectileMovement)
  (params (ImpactResult :type Hit%20Result%20Structure%20%28by%20ref%29) (ImpactVelocity :type Vector%20%28by%20ref%29 :default "0, 0, 0"))
  (if (<= (Variables|Default|GettimesCanBounce) (Variables|Default|GetcurrBounce))
    (Actor|DestroyActor)
    (else
      (bind _result (Math|Integer|IncrementInt (Variables|Default|GetcurrBounce))
        (:%20%20
          (Variables|Default|SetcurrBounce _result))))))

(event EventBeginPlay
  ;[1 1 1] Character and projectile cannot be on at the same time
  (Components|Activation|SetActive (Variables|Default|GetProjectileMovement) false false))

(event Collision|EventActorBeginOverlap
  (params (OtherActor :type Actor%20Object%20Reference)))

(event EventTick
  (params (DeltaSeconds :type Float%20%28single-precision%29)))

(event Collision|EventHit
  (params (MyComp :type Primitive%20Component%20Object%20Reference) (Other :type Actor%20Object%20Reference) (OtherComp :type Primitive%20Component%20Object%20Reference) (bSelfMoved :type Boolean) (HitLocation :type Vector :default "0, 0, 0") (HitNormal :type Vector :default "0, 0, 0") (NormalImpulse :type Vector :default "0, 0, 0") (Hit :type Hit%20Result%20Structure%20%28by%20ref%29))
  (bind _projectilemovement (Variables|Default|GetProjectileMovement))
  (if (Components|Activation|IsActive (Variables|Character|GetCharacterMovement))
    (Components|Activation|SetActive (Variables|Character|GetCharacterMovement) false false)
    (Variables|/Script/Engine.MovementComponent|SetVelocity _projectilemovement (* (* (Math|Vector|Normalize (- (Transformation|GetWorldLocation MyComp) (Transformation|GetWorldLocation OtherComp))) (Math|Conversions|ToVector(Float) 2e+03)) "1.000000,1.000000,0.000000"))
    (Components|Activation|SetActive _projectilemovement true false)))

(fn ConstructionScript)