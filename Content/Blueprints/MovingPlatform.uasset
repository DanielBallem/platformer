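; Moving platform actor that carries its static mesh along a spline, starting on BeginPlay or when hit by the third-person character, depending on exposed flags.
; A timeline, with play rate set from the completion time and optional looping, maps its track to distance along the spline.
; Each update sets the mesh's world location and optionally inherits spline rotation; the mesh's initial rotation always matches the spline start.
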(event OnComponentHit(StaticMesh)
  (params (HitComponent :type Primitive%20Component%20Object%20Reference) (OtherActor :type Actor%20Object%20Reference) (OtherComp :type Primitive%20Component%20Object%20Reference) (NormalImpulse :type Vector :default "0, 0, 0") (Hit :type Hit%20Result%20Structure%20%28by%20ref%29))
  (Utilities|Casting|CastToBP_ThirdPersonCharacter OtherActor)
  (if (Variables|Default|GetPlayerActivated)
    (CallFunction|MoveEvent)))

(event Custom|Move_Event
  (bind _move_object_t (Variables|Default|GetMove%20Object%20T))
  (bind _movementspline (Variables|Default|GetMovementSpline))
  (Components|Timeline|SetPlayRate _move_object_t (/ 1.0 (Variables|Default|GetTimeToCompleteInSec)))
  (Components|Timeline|SetLooping _move_object_t (Variables|Default|Getrepeat))
  (bind _movementtrack (Timeline|Move%20Object%20T Play)
    (:Update
      (if (Variables|Default|GetinheritSplineRotation)
        (Transformation|SetWorldLocationAndRotation (Variables|Default|GetStaticMesh) (Spline|GetLocationatDistanceAlongSpline _movementspline (Math|Float|Lerp 0.0 (Spline|GetSplineLength (Variables|Default|GetMovementSpline)) _movementtrack) "World") (Spline|GetRotationatDistanceAlongSpline _movementspline (Math|Float|Lerp 0.0 (Spline|GetSplineLength (Variables|Default|GetMovementSpline)) _movementtrack) "World") false false)
        (else
          (Transformation|SetWorldLocation (Variables|Default|GetStaticMesh) (Spline|GetLocationatDistanceAlongSpline _movementspline (Math|Float|Lerp 0.0 (Spline|GetSplineLength (Variables|Default|GetMovementSpline)) _movementtrack) "World") false false))))))

(event EventBeginPlay
  (|CallParentFunction)
  (Transformation|SetWorldRotation (Variables|Default|GetStaticMesh) (Spline|GetRotationatDistanceAlongSpline (Variables|Default|GetMovementSpline) 0.0 "World") false false)
  (if (Variables|Default|GetBeginOnPlay)
    (CallFunction|MoveEvent)))

(event Collision|EventActorBeginOverlap
  (params (OtherActor :type Actor%20Object%20Reference))
  (|CallParentFunction OtherActor) ; This node is disabled and will not be called.\nDrag off pins to build functionality.
)

(event EventTick
  (params (DeltaSeconds :type Float%20%28single-precision%29))
  (|CallParentFunction DeltaSeconds) ; This node is disabled and will not be called.\nDrag off pins to build functionality.
)

(fn ConstructionScript
  (|CallParentFunction))