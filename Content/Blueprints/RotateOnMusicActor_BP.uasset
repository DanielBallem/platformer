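; Mesh actor that rotates by a set increment each time its Triggered event fires, named for rotating to music.
; A timeline, its play rate scaled by RotationTime on BeginPlay, lerps the root's relative rotation from its current value by RotationPerEvent along the shortest path.
; An IsFiring flag ignores new triggers until the turn finishes.
; The construction script applies the configurable mesh.
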(event EventBeginPlay
  (Components|Timeline|SetPlayRate (Variables|Default|GetTurnTimeline) (/ 1.0 (Variables|Default|GetRotationTime))))

(event Collision|EventActorBeginOverlap
  (params (OtherActor :type Actor%20Object%20Reference)))

(event EventTick
  (params (DeltaSeconds :type Float%20%28single-precision%29)))

(event EventTriggered
  (if (not (Variables|Default|GetIsFiring))
    (Variables|Default|SetIsFiring true)
    (Variables|Default|SetcurrRotation (Variables|/Script/Engine.SceneComponent|GetRelativeRotation (Variables|Default|GetDefaultSceneRoot)))
    (bind _rotationcompletion (Timeline|TurnTimeline PlayFromStart)
      (:Update
        (Transformation|SetRelativeRotation (Variables|Default|GetDefaultSceneRoot) (Math|Rotator|Lerp(Rotator) (Variables|Default|GetcurrRotation) (Math|Rotator|CombineRotators (Variables|Default|GetcurrRotation) (Variables|Default|GetRotationPerEvent)) _rotationcompletion true) false false))
      (:Finished
        (Variables|Default|SetIsFiring false)))))

(fn ConstructionScript
  (Components|StaticMesh|SetStaticMesh (Variables|Default|GetStaticMesh) (Variables|Default|GetNew%20Mesh)))