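; Checkpoint actor that updates the respawn point when the third-person character enters its trigger.
; On BeginPlay it builds SpawnLocation from the root's world location plus the NewSpawnLocation offset, taking rotation directly from NewSpawnLocation and using unit scale.
; Overlapping CheckpointTrigger passes that transform to BP_ThirdPersonGameMode through SetRespawnTransform.
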(event OnComponentBeginOverlap(checkpointtrigger)
  (params (OverlappedComponent :type Primitive%20Component%20Object%20Reference) (OtherActor :type Actor%20Object%20Reference) (OtherComp :type Primitive%20Component%20Object%20Reference) (OtherBodyIndex :type Integer) (bFromSweep :type Boolean) (SweepResult :type Hit%20Result%20Structure%20%28by%20ref%29))
  (Utilities|Casting|CastToBP_ThirdPersonCharacter OtherActor)
  (bind _asbp_third_person_game_mode (Utilities|Casting|CastToBP_ThirdPersonGameMode (Game|GetGameMode)))
  (Default|SetRespawnTransform _asbp_third_person_game_mode (Variables|Default|GetspawnLocation)))

(event EventBeginPlay
  (bind _new_spawn_location (Variables|Default|Getnew%20spawn%20location))
  (Variables|Default|SetspawnLocation (Math|Transform|MakeTransform (+ (Transformation|GetWorldLocation (Variables|Default|GetDefaultSceneRoot)) (.location _new_spawn_location)) (.rotation _new_spawn_location) "1.000000,1.000000,1.000000")))

(event Collision|EventActorBeginOverlap
  (params (OtherActor :type Actor%20Object%20Reference)))

(event EventTick
  (params (DeltaSeconds :type Float%20%28single-precision%29)))

(fn ConstructionScript)