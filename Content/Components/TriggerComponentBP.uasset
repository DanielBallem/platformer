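; TriggerComponentBP is a trigger component that links to a referenced actor's TriggerableComponentBP so that it can fire that component.
; On BeginPlay it finds the component on TriggerableActorRef, caches it and calls RegisterTriggerEvent on it.
; TriggerOtherO later calls TriggeredEvent on the cached component without a validity check.
; A missing component is reported through AddExpectedLogError, an automation-test function, rather than an ordinary log.
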(event EventBeginPlay
  (CallFunction|RegisterwithTriggerO))

(event EventTick
  (params (DeltaSeconds :type Float%20%28single-precision%29)))

(fn TriggerOtherO
  (Default|TriggeredEvent (Variables|Default|GetTriggerableComponentReference)))

(fn RegisterwithTriggerO
  (bind _triggerableactorref (Variables|Default|GetTriggerableActorRef))
  (bind _returnvalue (Actor|GetComponentbyClass _triggerableactorref "/Game/Components/TriggerableComponentBP.TriggerableComponentBP_C"))
  (if (Utilities|IsValid _returnvalue)
    (bind _output_get (Variables|Default|SetTriggerableComponentReference _returnvalue))
    (Default|RegisterTriggerEvent _output_get)
    (else
      (Class|AutomationBlueprintFunctionLibrary|AddExpectedLogError "NOT TRIGGERABLE"))))