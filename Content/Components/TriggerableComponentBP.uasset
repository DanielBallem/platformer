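; Actor component that lets its owning actor respond to one or more triggers, relaying activations through TriggerInterfaceBP on that owner.
; Triggers register to raise a total count, and each activation increments a fired count.
; The owner receives Triggered until the count matches the total, when it receives TriggersCompleted instead.
; In alternating mode it skips counting and sends TriggerToggle on every activation.
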(event Custom|Triggered_Event
  (bind _returnvalue (Components|GetOwner))
  ;[1 1 1] alternating triggers will fire the toggle event
  ;
  ; Otherwise, it will fire trigger events until all associated triggers have been fired. It will fire a "triggersCompleted" event.
  (if (Variables|Default|GetAlternatingTrigger)
    (bind _astrigger_interface_bp (Utilities|Casting|CastToTriggerInterfaceBP (Components|GetOwner)))
    (Default|TriggerToggle _astrigger_interface_bp)
    (else
      (bind _output_get (Variables|Default|SetTriggeredSoFar (+ (Variables|Default|GetTriggeredSoFar) 1)))
      (if (== _output_get (stale Custom|RegisterTrigger_Event _output_get))
        (bind _astrigger_interface_bp_2 (Utilities|Casting|CastToTriggerInterfaceBP _returnvalue))
        (Default|TriggersCompleted _astrigger_interface_bp_2)
        (else
          (bind _astrigger_interface_bp_3 (Utilities|Casting|CastToTriggerInterfaceBP _returnvalue))
          (Default|Triggered _astrigger_interface_bp_3))))))

(event Custom|RegisterTrigger_Event
  ;[1 1 1] Counting how many triggers will be needed to complete all triggers
  (bind _output_get (Variables|Default|SetTotalTriggersRegistered (+ (Variables|Default|GetTotalTriggersRegistered) 1))))